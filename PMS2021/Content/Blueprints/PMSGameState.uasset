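; PMS game state that manages save data, checkpoints and the splash-screen flow for starting and reloading levels.
; Save functions load or create a PMSSaveData slot, and checkpoint updates swap the active checkpoint and write it to disk.
; It caches the PlayerHUD on BeginPlay; reloading shows the splash, waits briefly, then reopens the current level.
; StartOnInput binds to the SquidController's start dispatcher, and StartLevel unpauses and hides the splash.
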(event Custom|Reload%20Level
  (Default|ShowSplash (Variables|Default|GetHUD))
  (Utilities|FlowControl|Delay 0.5)
  (bind _returnvalue (Game|GetCurrentLevelName true))
  (Game|OpenLevel(byName) (Utilities|String|StringToName _returnvalue)))

(event EventBeginPlay
  (|InstantiateHUD_2))

(event EventTick
  (params (DeltaSeconds :type Float%20%28single-precision%29)))

(fn ConstructionScript)

(fn Load/CreateSave
  (params (SlotName :type String))
  (bind _returnvalue (SaveGame|LoadGamefromSlot SlotName))
  (Utilities|IsValid _returnvalue
    (:Is%20Valid
      (bind _aspmssave_data (Utilities|Casting|CastToPMSSaveData _returnvalue)
        (:then
          (Variables|Default|SetSaveState _aspmssave_data))
        (:CastFailed
          (bind _returnvalue_2 (SaveGame|CreateSaveGameObject "/Game/Blueprints/PMSSaveData.PMSSaveData_C" :!label _label))
          (Variables|Default|SetSaveState _returnvalue_2))))
    (:Is%20Not%20Valid
      (goto _label)))
  (return (Variables|Default|GetSaveState)))

(fn Create/OverrideSave
  (params (SlotName :type String))
  (bind _returnvalue (SaveGame|CreateSaveGameObject "/Game/Blueprints/PMSSaveData.PMSSaveData_C"))
  (bind _output_get (Variables|Default|SetSaveState _returnvalue))
  (SaveGame|SaveGametoSlot _output_get SlotName))

(fn UpdateCheckpoint
  (params (LastCheckpoint :type Checkpoint%20Object%20Reference))
  (bind _savestate (Variables|Default|GetSaveState))
  (Default|DeactivateCheckpoint (Variables|/Game/Blueprints/PMSSaveData.PMSSaveData_C|GetLastCheckpoint _savestate))
  (Default|ActivateCheckpoint LastCheckpoint)
  (Variables|/Game/Blueprints/PMSSaveData.PMSSaveData_C|SetLastCheckpoint _savestate LastCheckpoint)
  (SaveGame|SaveGametoSlot (Variables|Default|GetSaveState) (Variables|Default|GetSaveName)))

(fn StartonInput
  (bind _assquid_controller (Utilities|Casting|CastToSquidController (Game|GetPlayerController 0)))
  (EventDispatchers|BindEventtoStartLevelDispatch _assquid_controller (EventDispatchers|CreateEvent :!event StartLevel)))

(fn StartLevel
  (Game|SetGamePaused false)
  (Default|HideSplash (Variables|Default|GetHUD)))