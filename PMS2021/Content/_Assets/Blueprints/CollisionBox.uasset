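; CollisionBox is a toggleable hit box actor that applies damage on overlap, using its parent actor's instigator controller as the source.
; On overlap, a class check on the overlapped component's owner (the box's own side) selects Stun damage to the parent for CollisionBox, otherwise DamageType damage to damageable other actors.
; SetCollisionBox switches Box collision and Cube visibility together, and ToggleCollisionBox flips that state.
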(event OnComponentBeginOverlap(Box)
  (params (OverlappedComponent :type Primitive%20Component%20Object%20Reference) (OtherActor :type Actor%20Object%20Reference) (OtherComp :type Primitive%20Component%20Object%20Reference) (OtherBodyIndex :type Integer) (bFromSweep :type Boolean) (SweepResult :type Hit%20Result%20Structure%20%28by%20ref%29))
  (bind _returnvalue (Actor|GetParentActor))
  (bind _returnvalue_2 (Components|GetOwner OverlappedComponent))
  (bind _self self)
  (bind _instigator (Variables|/Script/Engine.Actor|GetInstigator _returnvalue))
  (bind _returnvalue_3 (Pawn|GetController _instigator))
  (if (not (== _returnvalue _returnvalue_2))
    (if (not (== OtherActor self))
      (if (== (Utilities|GetClass _returnvalue_2) "CollisionBox_C")
        (Game|Damage|ApplyDamage _returnvalue 1.0 _returnvalue_3 _self "/Game/_Assets/Blueprints/Stun.Stun_C")
        (elif (Variables|/Script/Engine.Actor|GetbCanBeDamaged OtherActor)
          (Game|Damage|ApplyDamage OtherActor 1.0 _returnvalue_3 _self "/Script/Engine.DamageType"))))))

(event EventBeginPlay)

(event Collision|EventActorBeginOverlap
  (params (OtherActor :type Actor%20Object%20Reference)))

(event EventTick
  (params (DeltaSeconds :type Float%20%28single-precision%29)))

(fn ConstructionScript)

(fn ToggleCollisionBox
  (CallFunction|SetCollisionBox (not (Variables|Default|GetEnabled))))

(fn SetCollisionBox
  (params (Enable :type Boolean))
  (Collision|SetCollisionEnabled (Variables|Default|GetBox) (select Enable "QueryAndPhysics" "NoCollision"))
  (Rendering|SetVisibility (Variables|Default|GetCube) Enable false)
  (Variables|Default|SetEnabled Enable))