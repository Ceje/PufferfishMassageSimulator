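; Game state Blueprint that manages save slots, checkpoints, streamed level instances, SFX volume and level restarts.
; Saves progress to PMSSaveData on checkpoint changes, while a separate MetaSave slot holds the current slot name and SFX volume, applied through a sound mix.
; Streaming requests are reference-counted per level, so an instance loads on first request and unloads on last release, though its map entry is never removed.
; The HUD splash covers reloads and hides on level start.
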(event Custom|StreamLevelRequest
  (params (Level :type Name) (SpawnTransform :type Transform))
  (bind (_location _rotation) (Math|Transform|BreakTransform SpawnTransform))
  (bind _levelrequests (Variables|Default|GetLevelRequests))
  (if (Utilities|Map|Contains _levelrequests Level)
    (bind _result (Math|Integer|IncrementInt (.Value (Utilities|Map|Find _levelrequests Level)))
      (:%20%20
        (Utilities|Map|Add _levelrequests Level _result)))
    (else
      (Utilities|Map|Add _levelrequests Level 1)
      (bind _returnvalue (Class|LevelStreamingDynamic|LoadLevelInstance (Utilities|String|ToString(Name) Level) _location _rotation))
      (Utilities|Map|Add (Variables|Default|GetLevelInstances) Level _returnvalue))))

(event Custom|UnstreamLevelRequest
  (params (Level :type Name))
  (bind _levelrequests (Variables|Default|GetLevelRequests))
  (bind _levelinstances (Variables|Default|GetLevelInstances))
  (bind (_value _returnvalue) (Utilities|Map|Find _levelrequests Level))
  (bind (_value_2 _returnvalue_2) (Utilities|Map|Find _levelinstances Level))
  (if _returnvalue
    (bind _result (Math|Integer|DecrementInt _value)
      (:%20%20
        (if (> _result 0)
          (Utilities|Map|Add _levelrequests Level _result)
          (else
            (Utilities|Map|Remove _levelrequests Level)
            (if _returnvalue_2 :!label _label
              (Class|LevelStreaming|SetIsRequestingUnloadandRemoval _value_2 true))))))
    (else
      (goto _label))))

(event Custom|Reload%20Level
  (Default|ShowSplash (Variables|Default|GetHUD))
  (Utilities|FlowControl|Delay 0.5)
  (bind _returnvalue (Game|GetCurrentLevelName true))
  (Game|OpenLevel(byName) (Utilities|String|StringToName _returnvalue)))

(event EventBeginPlay
  (CallFunction|LoadAudioLevels)
  (|InstantiateHUD_2))

(event EventTick
  (params (DeltaSeconds :type Float%20%28single-precision%29)))

(fn ConstructionScript)

(fn LoadSave
  (params (SlotName :type String))
  (bind _returnvalue (SaveGame|LoadGamefromSlot SlotName))
  (Utilities|IsValid _returnvalue
    (:Is%20Valid
      (bind _aspmssave_data (Utilities|Casting|CastToPMSSaveData _returnvalue)
        (:then
          (Variables|Default|SetSaveState _aspmssave_data)
          (Variables|Default|SetCurrentSave SlotName)
          (CallFunction|UpdateMetaSaveCurrentSave)
          (return (Variables|Default|GetSaveState)))
        (:CastFailed
          (Development|PrintString "Save Corrupted"))))
    (:Is%20Not%20Valid
      (Development|PrintString "No Save Found"))))

(fn CreateSave
  (params (SlotName :type String))
  (bind _returnvalue (SaveGame|CreateSaveGameObject "/Game/_Assets/Blueprints/SaveSystem/PMSSaveData.PMSSaveData_C"))
  (Variables|Default|SetSaveState _returnvalue)
  (Variables|Default|SetCurrentSave SlotName)
  (CallFunction|SaveGame))

(fn UpdateCheckpoint
  (params (LastCheckpoint :type Checkpoint%20Object%20Reference))
  (bind _savestate (Variables|Default|GetSaveState))
  (Utilities|IsValid (Variables|/Game/_Assets/Blueprints/SaveSystem/PMSSaveData.PMSSaveData_C|GetLastCheckpoint _savestate)
    (:Is%20Valid
      (Default|DeactivateCheckpoint (Variables|/Game/_Assets/Blueprints/SaveSystem/PMSSaveData.PMSSaveData_C|GetLastCheckpoint _savestate)))
    (:Is%20Not%20Valid
      _))
  (Default|ActivateCheckpoint LastCheckpoint)
  (Variables|/Game/_Assets/Blueprints/SaveSystem/PMSSaveData.PMSSaveData_C|SetLastCheckpoint _savestate LastCheckpoint)
  (CallFunction|SaveGame))

(fn StartonInput
  (bind _assquid_controller (Utilities|Casting|CastToSquidController (Game|GetPlayerController 0)))
  (EventDispatchers|BindEventtoStartLevelDispatch _assquid_controller (EventDispatchers|CreateEvent :!event StartLevel)))

(fn StartLevel
  (Game|SetGamePaused false)
  (Default|HideSplash (Variables|Default|GetHUD)))

(fn SaveGame
  (SaveGame|SaveGametoSlot (Variables|Default|GetSaveState) (Variables|Default|GetCurrentSave)))

(fn UpdateMetaSaveCurrentSave
  (bind _returnvalue (SaveGame|LoadGamefromSlot "MetaSave"))
  (bind _asmeta_save (Utilities|Casting|CastToMetaSave _returnvalue))
  (Variables|/Game/_Assets/Blueprints/SaveSystem/MetaSave.MetaSave_C|SetCurrentSave _asmeta_save (Variables|Default|GetCurrentSave))
  (SaveGame|SaveGametoSlot _asmeta_save "MetaSave"))

(fn GetStoredCurrentSave
  (bind _returnvalue (SaveGame|LoadGamefromSlot "MetaSave"))
  (bind _asmeta_save (Utilities|Casting|CastToMetaSave _returnvalue))
  (Development|PrintString (Variables|/Game/_Assets/Blueprints/SaveSystem/MetaSave.MetaSave_C|GetCurrentSave _asmeta_save))
  (return (Variables|/Game/_Assets/Blueprints/SaveSystem/MetaSave.MetaSave_C|GetCurrentSave _asmeta_save)))

(fn UpdateAudioLevels
  (Utilities|FlowControl|Sequence
    (:then_0
      (Class|GameplayStatics|ClearSoundMixClassOverride "/Game/_Assets/Blueprints/Sounds/NewSoundMix.NewSoundMix" "/Game/_Assets/Blueprints/Sounds/Effect.Effect" 1.0)
      (Audio|SetSoundMixClassOverride "/Game/_Assets/Blueprints/Sounds/NewSoundMix.NewSoundMix" "/Game/_Assets/Blueprints/Sounds/Effect.Effect" (Variables|Default|GetSFX%20Volume) 1.0 1.0 true))
    (:then_4
      (bind _returnvalue (SaveGame|LoadGamefromSlot "MetaSave"))
      (bind _asmeta_save (Utilities|Casting|CastToMetaSave _returnvalue))
      (Utilities|FlowControl|Sequence
        (:then_0
          (Variables|/Game/_Assets/Blueprints/SaveSystem/MetaSave.MetaSave_C|SetSFXVolume _asmeta_save (Variables|Default|GetSFX%20Volume)))
        (:then_5
          (SaveGame|SaveGametoSlot _asmeta_save "MetaSave"))))))

(fn LoadAudioLevels
  (Class|GameplayStatics|SetBaseSoundMix "/Game/_Assets/Blueprints/Sounds/NewSoundMix.NewSoundMix")
  (bind _returnvalue (SaveGame|LoadGamefromSlot "MetaSave"))
  (bind _asmeta_save (Utilities|Casting|CastToMetaSave _returnvalue))
  (Utilities|FlowControl|Sequence
    (:then_0
      (Variables|Default|SetSFX%20Volume (Variables|/Game/_Assets/Blueprints/SaveSystem/MetaSave.MetaSave_C|GetSFXVolume _asmeta_save)))
    (:then_5
      (CallFunction|UpdateAudioLevels))))