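; PMSPlayerState tracks the player's Stamina and TimePower meters, the resources tied to dashing and slowing time.
; Each Tick, StaminaRegen drains Stamina while Dashing and refills it otherwise, and TimeRegen does the same for TimePower based on TimeSlowed.
; TimeRegen divides by global time dilation so its rate holds in real time.
; Both meters are capped at a maximum, with no lower clamp here.
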(event EventBeginPlay)

(event EventTick
  (params (DeltaSeconds :type Float%20%28single-precision%29))
  (Utilities|FlowControl|Sequence
    (:then_0
      (|StaminaRegen DeltaSeconds))
    (:then_1
      (|TimeRegen DeltaSeconds))))

(fn ConstructionScript)