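; SquidController is a player controller that turns axis input into movement and aim for a Char1 pawn.
; On BeginPlay it caches the controlled Char1, or destroys itself if the pawn is another class.
; Both movement axis events run the same node, combining both axes into a vector rotated by the character's rotation for AddMovementInput.
; The aim axes feed directly into controller pitch and yaw.
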(event EventBeginPlay
  (bind _aschar_1 (Utilities|Casting|CastToChar1 (Pawn|GetControlledPawn))
    (:then
      (Variables|Default|SetChar1Ref _aschar_1))
    (:CastFailed
      (Actor|DestroyActor))))

(event Input|ActionEvents|InputActionAim
  (params (Key :type Key%20Structure :default "None")))

(event Input|ActionEvents|InputActionDodge
  (params (Key :type Key%20Structure :default "None")))

(event Input|AxisEvents|InputAxisForward/Backwards
  (params (AxisValue :type Float%20%28single-precision%29))
  (bind _char1ref (Variables|Default|GetChar1Ref))
  ;[1 1 1] Collect MOvement Input
  (Pawn|Input|AddMovementInput _char1ref (Math|Vector|RotateVector (Math|Conversions|ToVector(Vector2D) (Math|Vector2D|MakeVector2D (Input|AxisValues|GetForward/Backwards) (Input|AxisValues|GetLeft/Right))) (Transformation|GetActorRotation _char1ref)) 1e+02 false))

(event Input|AxisEvents|InputAxisHorizontalAim
  (params (AxisValue :type Float%20%28single-precision%29))
  (Class|PlayerController|AddYawInput AxisValue))

(event Input|AxisEvents|InputAxisVerticalAim
  (params (AxisValue :type Float%20%28single-precision%29))
  (Class|PlayerController|AddPitchInput AxisValue))

(event Input|AxisEvents|InputAxisLeft/Right
  (params (AxisValue :type Float%20%28single-precision%29))
  (bind _char1ref (Variables|Default|GetChar1Ref))
  ;[1 1 1] Collect MOvement Input
  (Pawn|Input|AddMovementInput _char1ref (Math|Vector|RotateVector (Math|Conversions|ToVector(Vector2D) (Math|Vector2D|MakeVector2D (Input|AxisValues|GetForward/Backwards) (Input|AxisValues|GetLeft/Right))) (Transformation|GetActorRotation _char1ref)) 1e+02 false))

(fn ConstructionScript)