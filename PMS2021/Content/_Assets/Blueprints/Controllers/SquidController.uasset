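; Player controller for Char1 that handles movement, look, pause, checkpoint use and a first-any-input level-start dispatch.
; Aim slows global time and scales camera post-process settings until release or until TimePower in the player state runs out.
; Dodge spends stamina on a short dash along control rotation plus input direction, clamping pitch while walking to avoid dashing into the ground.
; Each tick, a camera line cast toggles the HUD tooltip.
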(event EventPossess
  (params (PossessedPawn :type Pawn%20Object%20Reference))
  (bind _aschar_1 (Utilities|Casting|CastToChar1 PossessedPawn))
  (bind _output_get (Variables|Default|SetChar1Ref _aschar_1))
  (bind _aspmsgame_state (Utilities|Casting|CastToPMSGameState (Game|GetGameState)))
  (EventDispatchers|BindEventtoDeathDispatch _output_get (EventDispatchers|CreateEvent _aspmsgame_state :!event ReloadLevel)))

(event EventTick
  (params (DeltaSeconds :type Float%20%28single-precision%29))
  (Utilities|IsValid (Variables|Default|GetChar1Ref)
    (:Is%20Valid
      (Utilities|FlowControl|Sequence
        (:then_0
          (|CheckTimePower))
        (:then_1
          (|Show/HideTooltip))))))

(event EventBeginPlay
  (bind _aspmsplayer_state (Utilities|Casting|CastToPMSPlayerState (Variables|GetPlayerState)))
  (Variables|Default|SetPMSPlayerState _aspmsplayer_state)
  (bind _aspmsgame_state (Utilities|Casting|CastToPMSGameState (Game|GetGameState)))
  (Variables|Default|SetGameState _aspmsgame_state)
  (bind _asplayer_hud (Utilities|Casting|CastToPlayerHUD (HUD|GetHUD)))
  (Variables|Default|SetPlayerHud _asplayer_hud))

(event Input|ActionEvents|InputActionAim
  (params (Key :type Key%20Structure :default "None"))
  (:Pressed
    (CallFunction|SlowTime))
  (:Released
    (CallFunction|ResumeTime)))

(event Input|ActionEvents|InputActionDodge
  (params (Key :type Key%20Structure :default "None"))
  (bind _returnvalue (Pawn|GetControlRotation :!class /Script/Engine.Controller))
  (bind _pmsplayerstate (Variables|Default|GetPMSPlayerState))
  (bind _dash_cost (Variables|Default|GetDash%20Cost))
  (bind (_roll _pitch _yaw) (Math|Rotator|BreakRotator _returnvalue))
  ;[1 1 1] Dash Movement Function
  (:Pressed
    (if (>= (Variables|/Game/Blueprints/PMSPlayerState.PMSPlayerState_C|GetStamina _pmsplayerstate) _dash_cost)
      (Variables|/Game/Blueprints/PMSPlayerState.PMSPlayerState_C|SetStamina _pmsplayerstate (- (Variables|/Game/Blueprints/PMSPlayerState.PMSPlayerState_C|GetStamina _pmsplayerstate) _dash_cost))
      (Default|StartDash (Variables|Default|GetChar1Ref) (Math|Rotator|CombineRotators (Utilities|Select :Index (Variables|/Script/Engine.CharacterMovementComponent|GetMovementMode (Variables|/Script/Engine.Character|GetCharacterMovement (Variables|Default|GetChar1Ref))) :MOVE_None _returnvalue :MOVE_Walking (Math|Rotator|MakeRotator 0.0 (Math|Float|Max(Float) _pitch 0.0) _yaw) :MOVE_NavWalking _returnvalue :MOVE_Falling _returnvalue :MOVE_Swimming _returnvalue :MOVE_Flying _returnvalue :MOVE_Custom _returnvalue) (Math|Rotator|MakeRotfromX (Math|Vector|MakeVector (Input|AxisValues|GetForward/Backwards) (Input|AxisValues|GetLeft/Right) 0.0))))
      (Utilities|FlowControl|RetriggerableDelay 0.2)
      (Default|StopDash (Variables|Default|GetChar1Ref)))))

(event Input|ActionEvents|InputActionAnyInput
  (params (Key :type Key%20Structure :default "None"))
  (:Pressed
    (Default|CallStartLevelDispatch)
    (EventDispatchers|UnbindallEventsfromStartLevelDispatch)))

(event Input|ActionEvents|InputActionUseKey
  (params (Key :type Key%20Structure :default "None"))
  (:Pressed
    (bind _outhit (Default|CameraLineCast (Variables|Default|GetChar1Ref) (Utilities|Array|MakeArray "ObjectTypeQuery1") (Utilities|Array|MakeArray 0)))
    (bind _ascheckpoint (Utilities|Casting|CastToCheckpoint (.HitActor (Collision|BreakHitResult _outhit))))
    (Default|UpdateCheckpoint (Variables|Default|GetGameState) _ascheckpoint)))

(event Input|ActionEvents|InputActionPause
  (params (Key :type Key%20Structure :default "None"))
  (:Pressed
    (Default|Pause (Variables|Default|GetPlayerHud))))

(event Input|AxisEvents|InputAxisForward/Backwards
  (params (AxisValue :type Float%20%28single-precision%29))
  (bind _char1ref (Variables|Default|GetChar1Ref))
  ;[1 1 1] Collect Movement Input
  (Utilities|IsValid _char1ref
    (:Is%20Valid
      (Pawn|Input|AddMovementInput _char1ref (Math|Vector|RotateVector (Math|Conversions|ToVector(Vector2D) (Math|Vector2D|MakeVector2D (Input|AxisValues|GetForward/Backwards) (Input|AxisValues|GetLeft/Right))) (Transformation|GetActorRotation _char1ref)) 1e+02 false))))

(event Input|AxisEvents|InputAxisHorizontalAim
  (params (AxisValue :type Float%20%28single-precision%29))
  (Class|PlayerController|AddYawInput AxisValue))

(event Input|AxisEvents|InputAxisVerticalAim
  (params (AxisValue :type Float%20%28single-precision%29))
  (bind _result (Math|Float|NegateFloat AxisValue)
    (:%20%20
      (Class|PlayerController|AddPitchInput _result))))

(event Input|AxisEvents|InputAxisLeft/Right
  (params (AxisValue :type Float%20%28single-precision%29))
  (bind _char1ref (Variables|Default|GetChar1Ref))
  ;[1 1 1] Collect Movement Input
  (Utilities|IsValid _char1ref
    (:Is%20Valid
      (Pawn|Input|AddMovementInput _char1ref (Math|Vector|RotateVector (Math|Conversions|ToVector(Vector2D) (Math|Vector2D|MakeVector2D (Input|AxisValues|GetForward/Backwards) (Input|AxisValues|GetLeft/Right))) (Transformation|GetActorRotation _char1ref)) 1e+02 false))))

(fn ConstructionScript)

(fn SlowTime
  (bind _char1ref (Variables|Default|GetChar1Ref))
  (bind _camera (Variables|/Game/_Assets/Blueprints/Characters/Char1.Char1_C|GetCamera _char1ref))
  (bind _postprocesssettings (Variables|/Script/Engine.CameraComponent|GetPostProcessSettings _camera))
  (bind (_motionbluramount _motionblurmax) (Utilities|Struct|BreakPostProcessSettings _postprocesssettings))
  (Variables|/Game/Blueprints/PMSPlayerState.PMSPlayerState_C|SetTimeSlowed (Variables|Default|GetPMSPlayerState) true)
  (Utilities|Time|SetGlobalTimeDilation 0.1)
  (Utilities|Struct|SetmembersinPostProcessSettings _postprocesssettings (* _motionbluramount 0.1) (* _motionblurmax 0.1)))

(fn ResumeTime
  (bind _char1ref (Variables|Default|GetChar1Ref))
  (bind _camera (Variables|/Game/_Assets/Blueprints/Characters/Char1.Char1_C|GetCamera _char1ref))
  (bind _postprocesssettings (Variables|/Script/Engine.CameraComponent|GetPostProcessSettings _camera))
  (bind (_motionbluramount _motionblurmax) (Utilities|Struct|BreakPostProcessSettings _postprocesssettings))
  (Variables|/Game/Blueprints/PMSPlayerState.PMSPlayerState_C|SetTimeSlowed (Variables|Default|GetPMSPlayerState) false)
  (Utilities|Time|SetGlobalTimeDilation 1.0)
  (Variables|/Script/Engine.Actor|SetCustomTimeDilation (Pawn|GetControlledPawn) 1.0)
  (Utilities|Struct|SetmembersinPostProcessSettings _postprocesssettings (* _motionbluramount 1.0) (* _motionblurmax 1.0)))