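; Base AI controller for Cube enemies that detects the player and spreads an alarm to other listeners.
; On BeginPlay it runs the Base behavior tree and binds PawnSensing sight and hearing.
; Sighting the player in certain Cube states sets an alerted state and the PlayerActor blackboard key, emitting an "Alarm" noise if not already alerted.
; Any heard noise applies the same state and targets player zero, without checking tag or instigator.
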(event Custom|HearAlarm
  (params (Instigator :type Pawn%20Object%20Reference) (Location :type Vector%20%28by%20ref%29) (Volume :type Float%20%28single-precision%29))
  (bind _ascube (Utilities|Casting|CastToCube (Pawn|GetControlledPawn)))
  (Variables|/Game/_Assets/Blueprints/Characters/Cube.Cube_C|SetState _ascube "NewEnumerator8")
  (AI|Components|Blackboard|SetValueasObject (AI|GetBlackboard self) (Utilities|Name|MakeLiteralName "PlayerActor") (Game|Player|GetPlayerPawn 0)))

(event EventBeginPlay
  (bind _pawnsensing (Variables|Default|GetPawnSensing))
  (AI|RunBehaviorTree "/Game/_Assets/Blueprints/AI/Base.Base")
  (EventDispatchers|BindEventtoOnSeePawn _pawnsensing (delegate SpotPlayer))
  (EventDispatchers|BindEventtoOnHearNoise _pawnsensing (delegate Custom|HearAlarm)))

(event EventTick
  (params (DeltaSeconds :type Float%20%28single-precision%29)))

(fn ConstructionScript)

(event Custom|SeePlayer
  (params (Pawn :type Pawn%20Object%20Reference))
  (bind _returnvalue (Pawn|GetControlledPawn))
  (if (== Pawn (Game|Player|GetPlayerPawn 0))
    (bind _ascube (Utilities|Casting|CastToCube _returnvalue)
      (:then
        (if (Utilities|Array|ContainsItem (Utilities|Array|MakeArray "NewEnumerator3" "NewEnumerator8" "NewEnumerator6" "NewEnumerator9") (Variables|/Game/_Assets/Blueprints/Characters/Cube.Cube_C|GetState _ascube))
          (if (Utilities|Enum|Equal(Enum) (Variables|/Game/_Assets/Blueprints/Characters/Cube.Cube_C|GetState _ascube) "NewEnumerator8")
            _
            (else
              (Class|Actor|MakeNoise 1.0 _returnvalue (Transformation|GetActorLocation _returnvalue) 1e+04 "Alarm")))
          (Variables|/Game/_Assets/Blueprints/Characters/Cube.Cube_C|SetState _ascube "NewEnumerator8")
          (AI|Components|Blackboard|SetValueasObject (AI|GetBlackboard self) (Utilities|Name|MakeLiteralName "PlayerActor") Pawn)
          (Development|PrintString "PlayerSpotted")))
      (:CastFailed
        (Development|PrintString "Bad Enemy Cast (Spot Player)")))))