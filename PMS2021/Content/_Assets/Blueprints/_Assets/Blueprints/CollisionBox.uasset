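; CollisionBox is a toggleable hitbox actor that deals damage on overlap and acts on behalf of its parent actor.
; Box overlaps ignore the parent, deal light damage to damageable actors, and deal heavy Stun damage when the other component belongs to another CollisionBox.
; Damage the box receives is forwarded to the parent, so clashing boxes pass stuns to their owners.
; SetCollisionBox and ToggleCollisionBox switch collision and cube visibility together.
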(event OnComponentBeginOverlap(Box)
  (params (OverlappedComponent :type Primitive%20Component%20Object%20Reference) (OtherActor :type Actor%20Object%20Reference) (OtherComp :type Primitive%20Component%20Object%20Reference) (OtherBodyIndex :type Integer) (bFromSweep :type Boolean) (SweepResult :type Hit%20Result%20Structure%20%28by%20ref%29))
  (bind _self self)
  (Utilities|IsValid OtherActor
    (:Is%20Valid
      (if (not (== (Actor|GetParentActor) OtherActor))
        (if (== (Utilities|GetClass (Components|GetOwner OtherComp)) "CollisionBox_C")
          (Game|Damage|ApplyDamage OtherActor 1e+03 0 _self "/Game/_Assets/Blueprints/Enum/Stun.Stun_C")
          (elif (Variables|/Script/Engine.Actor|GetbCanBeDamaged OtherActor)
            (Game|Damage|ApplyDamage OtherActor 1.0 0 _self "/Script/Engine.DamageType")))))))

(event EventBeginPlay)

(event Collision|EventActorBeginOverlap
  (params (OtherActor :type Actor%20Object%20Reference)))

(event EventTick
  (params (DeltaSeconds :type Float%20%28single-precision%29)))

(event Game|Damage|EventAnyDamage
  (params (Damage :type Float%20%28single-precision%29) (DamageType :type Damage%20Type%20Object%20Reference) (InstigatedBy :type Controller%20Object%20Reference) (DamageCauser :type Actor%20Object%20Reference))
  (bind _returnvalue (Actor|GetParentActor))
  (Utilities|IsValid _returnvalue
    (:Is%20Valid
      (Game|Damage|ApplyDamage _returnvalue Damage InstigatedBy DamageCauser (Utilities|GetClass DamageType)))))

(fn ConstructionScript)

(fn ToggleCollisionBox
  (CallFunction|SetCollisionBox (not (Variables|Default|GetEnabled))))

(fn SetCollisionBox
  (params (Enable :type Boolean))
  (Collision|SetCollisionEnabled (Variables|Default|GetBox) (select Enable "QueryAndPhysics" "NoCollision"))
  (Rendering|SetVisibility (Variables|Default|GetCube) Enable false)
  (Variables|Default|SetEnabled Enable))