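; Player character with a camera-based reach trace and a high-speed dash fronted by a child-actor collision box.
; Dashing switches to Flying, forces velocity each tick and rotates the box toward the dash direction until stopped.
; Stun damage cancels the dash and launches the character away from the causer, scaled by damage; other damage destroys it.
; Trace reach derives from spring arm length, actor bounds and base reach at construction.
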(event Game|Damage|EventAnyDamage
  (params (Damage :type Float%20%28single-precision%29) (DamageType :type Damage%20Type%20Object%20Reference) (InstigatedBy :type Controller%20Object%20Reference) (DamageCauser :type Actor%20Object%20Reference))
  (bind _returnvalue (Transformation|GetActorLocation DamageCauser))
  (bind _returnvalue_2 (Transformation|GetActorLocation))
  (bind _returnvalue_3 (Math|Rotator|FindLookatRotation _returnvalue _returnvalue_2))
  (bind (_roll _pitch _yaw) (Math|Rotator|BreakRotator _returnvalue_3))
  (if (== (Utilities|GetClass DamageType) "/Game/_Assets/Blueprints/Enum/Stun.Stun_C")
    (CallFunction|StopDash)
    (Character|LaunchCharacter (* (Math|Vector|GetForwardVector (Math|Rotator|MakeRotator _roll 45.0 _yaw)) Damage) true true)
    (else
      (Default|CallDeathDispatch)
      (Actor|DestroyActor))))

(event EventDestroyed
  (Input|DisableInput (Game|GetPlayerController 0)))

(event EventTick
  (params (DeltaSeconds :type Float%20%28single-precision%29))
  (if (Variables|Default|GetDashing)
    (Variables|/Script/Engine.MovementComponent|SetVelocity (Variables|Character|GetCharacterMovement) (Variables|Default|GetDashVelocity))))

(event EventBeginPlay
  (bind _ascollision_box (Utilities|Casting|CastToCollisionBox (Variables|/Script/Engine.ChildActorComponent|GetChildActor (Variables|Default|GetChildActor))))
  (bind _output_get (Variables|Default|SetCollision%20Box _ascollision_box))
  (Default|SetCollisionBox _output_get false)
  (Class|AudioMixerBlueprintLibrary|PrimeSoundCueforPlayback "/Game/_Assets/Blueprints/Sounds/HitSound.HitSound"))

(fn ConstructionScript
  (|SetCharacterReach_2))

(fn StopDash
  (bind _charactermovement (Variables|Character|GetCharacterMovement))
  (if (Variables|Default|GetDashing)
    (Default|SetCollisionBox (Variables|Default|GetCollision%20Box) false)
    (Variables|/Script/Engine.MovementComponent|SetVelocity _charactermovement "0, 0, 0")
    (Pawn|Components|CharacterMovement|SetMovementMode _charactermovement "MOVE_Walking" 0)
    (Variables|Default|SetDashing false)
    (Variables|Default|SetbUseControllerRotationYaw true)
    (Default|CallStopDashDispatch)))

(fn StartDash
  (params (InRot :type Rotator))
  (if (not (Variables|Default|GetDashing))
    (Variables|Default|SetDashing true)
    (CallFunction|SetBarrierFacing InRot)
    (Default|SetCollisionBox (Variables|Default|GetCollision%20Box) true)
    (Pawn|Components|CharacterMovement|SetMovementMode (Variables|Character|GetCharacterMovement) "MOVE_Flying" 0)
    (Variables|Default|SetDashVelocity (* (Math|Vector|GetForwardVector InRot) 5e+03))
    (Variables|Default|SetbUseControllerRotationYaw false)
    (Default|CallStartDashDispatch)))

(fn CameraLineCast
  (params (ObjectTypes :type Array%20of%20EObjectTypeQuery%20Enums :default "ObjectTypeQuery1") (ActorsToIgnore :type Array%20of%20Actor%20Object%20References))
  (bind _camera (Variables|Default|GetCamera))
  (bind _returnvalue (Transformation|GetWorldLocation _camera))
  (bind (_outhit _returnvalue_2) (Collision|LineTraceForObjects _returnvalue (+ _returnvalue (* (Math|Vector|GetForwardVector _camera) (Variables|Default|GetCharacter%20Reach))) ObjectTypes false ActorsToIgnore "None"))
  (return _outhit _returnvalue_2))

(fn SetBarrierFacing
  (params (Direction :type Rotator))
  (bind _childactor (Variables|Default|GetChildActor))
  (bind _capsulecomponent (Variables|Collision|GetCapsuleComponent))
  (bind _returnvalue (Transformation|GetWorldRotation _capsulecomponent))
  (bind _returnvalue_2 (Class|KismetMathLibrary|NegateRotator _returnvalue))
  (bind _returnvalue_3 (Math|Rotator|CombineRotators Direction _returnvalue_2))
  (Transformation|SetRelativeLocationAndRotation _childactor (* (Math|Vector|GetForwardVector _returnvalue_3) (Math|Vector|VectorLength (Variables|/Script/Engine.SceneComponent|GetRelativeLocation _childactor))) _returnvalue_3 false false))