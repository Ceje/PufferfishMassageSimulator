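; Player controller for the Char1 pawn, turning input into movement, aiming, dashing, global slow-motion, pausing and level start.
; On possess it caches the pawn and binds its dash and death dispatchers, mirroring dash state to PMSPlayerState with a short post-dash lockout.
; Tick ends dash or slow-motion when stamina or time power runs out.
; Camera line casts drive HUD tooltips and let the Use key update the game state's checkpoint.
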(event Custom|Start%20Dash%20Relay
  (Variables|/Game/_Assets/Blueprints/PMSPlayerState.PMSPlayerState_C|SetDashing (Variables|Default|GetPMSPlayerState) true)
  (Variables|Default|SetDashLag true))

(event Custom|Stop%20Dash%20Relay
  (Variables|/Game/_Assets/Blueprints/PMSPlayerState.PMSPlayerState_C|SetDashing (Variables|Default|GetPMSPlayerState) false)
  (Utilities|FlowControl|Delay 0.4)
  (Variables|Default|SetDashLag false))

(event EventPossess
  (params (PossessedPawn :type Pawn%20Object%20Reference))
  (bind _char1ref (Variables|Default|GetChar1Ref))
  (Utilities|FlowControl|Sequence
    (:then_0
      (|RecordPawn PossessedPawn))
    (:then_1
      (EventDispatchers|BindEventtoStartDashDispatch _char1ref (delegate Custom|Start%20Dash%20Relay))
      (EventDispatchers|BindEventtoStopDashDispatch _char1ref (delegate Custom|Stop%20Dash%20Relay)))))

(event EventTick
  (params (DeltaSeconds :type Float%20%28single-precision%29))
  (Utilities|IsValid (Variables|Default|GetChar1Ref)
    (:Is%20Valid
      (Utilities|FlowControl|Sequence
        (:then_0
          (|CheckTimePower))
        (:then_1
          (|Show/HideTooltip))
        (:then_2
          (|CheckDashPower))))))

(event EventBeginPlay
  (bind _aspmsplayer_state (Utilities|Casting|CastToPMSPlayerState (Variables|GetPlayerState)))
  (Variables|Default|SetPMSPlayerState _aspmsplayer_state)
  (bind _aspmsgame_state (Utilities|Casting|CastToPMSGameState (Game|GetGameState)))
  (Variables|Default|SetGameState _aspmsgame_state)
  (bind _asplayer_hud (Utilities|Casting|CastToPlayerHUD (HUD|GetHUD)))
  (Variables|Default|SetPlayerHud _asplayer_hud))

(event Input|ActionEvents|InputActionAim
  (params (Key :type Key%20Structure))
  (:Pressed
    (CallFunction|SlowTime))
  (:Released
    (CallFunction|ResumeTime)))

(event Input|ActionEvents|InputActionDodge
  (params (Key :type Key%20Structure))
  (bind _char1ref (Variables|Default|GetChar1Ref))
  (:Pressed
    (if (not (Variables|Default|GetDashLag))
      (Utilities|IsValid _char1ref
        (:Is%20Valid
          (Default|StartDash _char1ref (|CalculateDashRotation))))))
  (:Released
    (Utilities|IsValid _char1ref
      (:Is%20Valid
        (Default|StopDash _char1ref)))))

(event Input|ActionEvents|InputActionAnyInput
  (params (Key :type Key%20Structure))
  (:Pressed
    (Default|CallStartLevelDispatch)
    (EventDispatchers|UnbindallEventsfromStartLevelDispatch)))

(event Input|ActionEvents|InputActionUseKey
  (params (Key :type Key%20Structure))
  (:Pressed
    (bind _outhit (Default|CameraLineCast (Variables|Default|GetChar1Ref) (Utilities|Array|MakeArray "ObjectTypeQuery1") (Utilities|Array|MakeArray 0)))
    (bind _ascheckpoint (Utilities|Casting|CastToCheckpoint (.HitActor (Collision|BreakHitResult _outhit))))
    (Default|UpdateCheckpoint (Variables|Default|GetGameState) _ascheckpoint)))

(event Input|ActionEvents|InputActionPause
  (params (Key :type Key%20Structure))
  (:Pressed
    (Default|Pause (Variables|Default|GetPlayerHud))))

(event Input|AxisEvents|InputAxisForward/Backwards
  (params (AxisValue :type Float%20%28single-precision%29))
  (bind _char1ref (Variables|Default|GetChar1Ref))
  ;[1 1 1] Collect Movement Input
  (Utilities|IsValid _char1ref
    (:Is%20Valid
      (Pawn|Input|AddMovementInput _char1ref (Math|Vector|RotateVector (Math|Conversions|ToVector(Vector2D) (Math|Vector2D|MakeVector2D (Input|AxisValues|GetForward/Backwards) (Input|AxisValues|GetLeft/Right))) (Transformation|GetActorRotation _char1ref)) 1e+02 false))))

(event Input|AxisEvents|InputAxisHorizontalAim
  (params (AxisValue :type Float%20%28single-precision%29))
  (Class|PlayerController|AddYawInput AxisValue))

(event Input|AxisEvents|InputAxisVerticalAim
  (params (AxisValue :type Float%20%28single-precision%29))
  (bind _result (Math|Float|NegateFloat AxisValue)
    (:%20%20
      (Class|PlayerController|AddPitchInput _result))))

(event Input|AxisEvents|InputAxisLeft/Right
  (params (AxisValue :type Float%20%28single-precision%29))
  (bind _char1ref (Variables|Default|GetChar1Ref))
  ;[1 1 1] Collect Movement Input
  (Utilities|IsValid _char1ref
    (:Is%20Valid
      (Pawn|Input|AddMovementInput _char1ref (Math|Vector|RotateVector (Math|Conversions|ToVector(Vector2D) (Math|Vector2D|MakeVector2D (Input|AxisValues|GetForward/Backwards) (Input|AxisValues|GetLeft/Right))) (Transformation|GetActorRotation _char1ref)) 1e+02 false))))

(fn ConstructionScript)

(fn SlowTime
  (bind _char1ref (Variables|Default|GetChar1Ref))
  (bind _camera (Variables|/Game/_Assets/Blueprints/Characters/Char1.Char1_C|GetCamera _char1ref))
  (bind _postprocesssettings (Variables|/Script/Engine.CameraComponent|GetPostProcessSettings _camera))
  (bind (_motionbluramount _motionblurmax) (Utilities|Struct|BreakPostProcessSettings _postprocesssettings))
  (Variables|/Game/_Assets/Blueprints/PMSPlayerState.PMSPlayerState_C|SetTimeSlowed (Variables|Default|GetPMSPlayerState) true)
  (Utilities|Time|SetGlobalTimeDilation 0.1)
  (Utilities|Struct|SetmembersinPostProcessSettings _postprocesssettings (* _motionbluramount 0.1) (* _motionblurmax 0.1)))

(fn ResumeTime
  (bind _char1ref (Variables|Default|GetChar1Ref))
  (bind _camera (Variables|/Game/_Assets/Blueprints/Characters/Char1.Char1_C|GetCamera _char1ref))
  (bind _postprocesssettings (Variables|/Script/Engine.CameraComponent|GetPostProcessSettings _camera))
  (bind (_motionbluramount _motionblurmax) (Utilities|Struct|BreakPostProcessSettings _postprocesssettings))
  (Variables|/Game/_Assets/Blueprints/PMSPlayerState.PMSPlayerState_C|SetTimeSlowed (Variables|Default|GetPMSPlayerState) false)
  (Utilities|Time|SetGlobalTimeDilation 1.0)
  (Variables|/Script/Engine.Actor|SetCustomTimeDilation (Pawn|GetControlledPawn) 1.0)
  (Utilities|Struct|SetmembersinPostProcessSettings _postprocesssettings (* _motionbluramount 1.0) (* _motionblurmax 1.0)))