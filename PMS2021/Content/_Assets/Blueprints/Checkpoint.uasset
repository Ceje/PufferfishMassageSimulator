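; Checkpoint actor that shows whether it is active through a spotlight color and a mesh material.
; ActivateCheckpoint sets a pale cyan light and the active material, while DeactivateCheckpoint sets a green light and the inactive material.
; It starts deactivated on BeginPlay and has no working overlap or tick logic, so nothing inside the asset triggers activation.
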(event Collision|EventActorBeginOverlap
  (params (OtherActor :type Actor%20Object%20Reference)))

(event EventTick
  (params (DeltaSeconds :type Float%20%28single-precision%29)))

(event EventBeginPlay
  (CallFunction|DeactivateCheckpoint))

(fn ConstructionScript)

(fn ActivateCheckpoint
  (Rendering|Components|Light|SetLightColor (Variables|Default|GetSpotLight) (Math|Color|MakeColor 0.486 0.788 0.82) true)
  (Rendering|Material|SetMaterial (Variables|Default|GetStaticMesh) 0 "/Game/_Assets/Blueprints/Models/Check_point/ActiveCheckpointMaterial.ActiveCheckpointMaterial"))

(fn DeactivateCheckpoint
  (Rendering|Components|Light|SetLightColor (Variables|Default|GetSpotLight) (Class|KismetMathLibrary|LinearColorGreen) true)
  (Rendering|Material|SetMaterial (Variables|Default|GetStaticMesh) 0 "/Game/_Assets/Blueprints/Models/Check_point/InactiveCheckpoint.InactiveCheckpoint"))