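; Enemy spawner actor that, while active, periodically spawns enemies from its class list at its own transform.
; Tick runs a countdown gate with randomized interval variance, then a gate that allows infinite spawns or deactivates the spawner once a finite count runs out.
; Passing both gates spawns either a random class or the next entry in a looping index pattern.
; Separate functions also spawn by pattern index or given class.
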(event EventBeginPlay)

(event Collision|EventActorBeginOverlap
  (params (OtherActor :type Actor%20Object%20Reference)))

(event EventTick
  (params (DeltaSeconds :type Float%20%28single-precision%29))
  (if (Variables|Default|GetSpawnActive)
    (|TimerGate DeltaSeconds)
    (|SpawnGate)
    (switch Utilities|FlowControl|Switch|SwitchonSpawnerType (Variables|Default|GetType)
      (:NewEnumerator0
        (CallFunction|SpawnRandom))
      (:NewEnumerator1
        (CallFunction|SpawnbyPattern)))))

(fn ConstructionScript)

(fn SpawnbyPattern
  (bind _spawnpattern (Variables|Default|GetSpawnPattern))
  (if (<= (Utilities|Array|Length (Variables|Default|GetSpawnPattern)) (Variables|Default|GetSpawnPatternIndex))
    (Variables|Default|SetSpawnPatternIndex 0))
  (if (Utilities|Array|IsValidIndex _spawnpattern (Variables|Default|GetSpawnPatternIndex))
    (Game|SpawnActorfromClass (Utilities|Array|Get(acopy) (Variables|Default|GetEnemyTypes) (Utilities|Array|Get(acopy) _spawnpattern (Variables|Default|GetSpawnPatternIndex))) (Transformation|GetActorTransform) "AdjustIfPossibleButAlwaysSpawn" 0 0)
    (Math|Integer|IncrementInt (Variables|Default|GetSpawnPatternIndex))))

(fn SpawnRandom
  (bind _enemytypes (Variables|Default|GetEnemyTypes))
  (Game|SpawnActorfromClass (Utilities|Array|Get(acopy) _enemytypes (Math|Random|RandomIntegerinRange 0 (- (Utilities|Array|Length _enemytypes) 1))) (Transformation|GetActorTransform) "AdjustIfPossibleButAlwaysSpawn" 0 0))

(fn SpawnbyIndex
  (params (SpawnIndex :type Integer))
  (bind _spawnpattern (Variables|Default|GetSpawnPattern))
  (if (Utilities|Array|IsValidIndex _spawnpattern SpawnIndex)
    (Game|SpawnActorfromClass (Utilities|Array|Get(acopy) (Variables|Default|GetEnemyTypes) (Utilities|Array|Get(acopy) _spawnpattern SpawnIndex)) (Transformation|GetActorTransform) "AdjustIfPossibleButAlwaysSpawn" 0 0)))

(fn SpawnbyClass
  (params (Class :type Actor%20Class%20Reference))
  (Game|SpawnActorfromClass Class (Transformation|GetActorTransform) "AdjustIfPossibleButAlwaysSpawn" 0 0))