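; Behavior tree task that runs a timed cooldown on an AI-controlled Cube pawn.
; On execute it caches the Cube and switches its state enum, failing with a debug print if the controller or pawn cast fails.
; Tick accumulates time for about two seconds, then sets a second state, resets the timer and succeeds; abort does the same switch and reset.
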(event EventReceiveExecute
  (params (OwnerActor :type Actor%20Object%20Reference))
  (bind _asaicontroller (Utilities|Casting|CastToAIController OwnerActor)
    (:then
      (bind _ascube (Utilities|Casting|CastToCube (Pawn|GetControlledPawn _asaicontroller))
        (:then
          (bind _output_get (Variables|Default|SetActor _ascube))
          (Variables|/Game/_Assets/Blueprints/Characters/Cube.Cube_C|SetState _output_get "NewEnumerator2"))
        (:CastFailed
          (Development|PrintString "bad pawn")
          (AI|BehaviorTree|FinishExecute false :!label _label))))
    (:CastFailed
      (Development|PrintString "bad parent")
      (goto _label))))

(event EventTick
  (params (OwnerActor :type Actor%20Object%20Reference) (DeltaSeconds :type Float%20%28single-precision%29))
  (if (> (Variables|Default|GetCooldown%20Timer) 2.0)
    (Variables|/Game/_Assets/Blueprints/Characters/Cube.Cube_C|SetState (Variables|Default|GetActor) "NewEnumerator3")
    (Variables|Default|SetCooldown%20Timer 0.0)
    (AI|BehaviorTree|FinishExecute true)
    (else
      (Variables|Default|SetCooldown%20Timer (+ DeltaSeconds (Variables|Default|GetCooldown%20Timer))))))

(event EventReceiveAbort
  (params (OwnerActor :type Actor%20Object%20Reference))
  (Variables|/Game/_Assets/Blueprints/Characters/Cube.Cube_C|SetState (Variables|Default|GetActor) "NewEnumerator3")
  (Variables|Default|SetCooldown%20Timer 0.0)
  (Class|BTTaskBlueprintBase|FinishAbort))