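; Behavior tree service that copies the controlled Cube pawn's State into a Blackboard enum key.
; On activation and on each tick, it casts the owner to an AIController and its pawn to Cube, then writes the State to the Key selector.
; The write is skipped if either cast fails.
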(event EventTick
  (params (OwnerActor :type Actor%20Object%20Reference) (DeltaSeconds :type Float%20%28single-precision%29))
  (bind _asaicontroller (Utilities|Casting|CastToAIController OwnerActor))
  (bind _ascube (Utilities|Casting|CastToCube (Pawn|GetControlledPawn _asaicontroller)))
  (Class|BTFunctionLibrary|SetBlackboardValueasEnum (Variables|Default|GetKey) (Variables|/Game/_Assets/Blueprints/Characters/Cube.Cube_C|GetState _ascube)))

(event EventReceiveActivation
  (params (OwnerActor :type Actor%20Object%20Reference))
  (bind _asaicontroller (Utilities|Casting|CastToAIController OwnerActor))
  (bind _ascube (Utilities|Casting|CastToCube (Pawn|GetControlledPawn _asaicontroller)))
  (Class|BTFunctionLibrary|SetBlackboardValueasEnum (Variables|Default|GetKey) (Variables|/Game/_Assets/Blueprints/Characters/Cube.Cube_C|GetState _ascube)))