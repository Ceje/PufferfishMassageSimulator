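; Behavior tree service that picks the next patrol node for an AI-controlled Cube when activated.
; It increments the pawn's PathingTarget and writes that PatrolPath entry to a Blackboard key.
; When the entry is invalid, the index resets and PathingStyle decides whether to reverse the path, teleport to the first node, or loop.
; Any other style changes the pawn's State instead of setting a target.
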(event EventReceiveActivation
  (params (OwnerActor :type Actor%20Object%20Reference))
  (bind _asbase_aicontroller (Utilities|Casting|CastToBaseAIController OwnerActor))
  (bind _ascube (Utilities|Casting|CastToCube (Pawn|GetControlledPawn _asbase_aicontroller)))
  (bind _result (Math|Integer|IncrementInt (Variables|/Game/_Assets/Blueprints/Characters/Cube.Cube_C|GetPathingTarget _ascube))
    (:%20%20
      (Utilities|IsValid (Utilities|Array|Get(acopy) (Variables|/Game/_Assets/Blueprints/Characters/Cube.Cube_C|GetPatrolPath _ascube) _result)
        (:Is%20Valid
          (Class|BTFunctionLibrary|SetBlackboardValueasObject (Variables|Default|GetKey) (Utilities|Array|Get(acopy) (Variables|/Game/_Assets/Blueprints/Characters/Cube.Cube_C|GetPatrolPath _ascube) _result)))
        (:Is%20Not%20Valid
          (bind _output_get (Variables|/Game/_Assets/Blueprints/Characters/Cube.Cube_C|SetPathingTarget _ascube 0))
          (if (Utilities|Enum|Equal(Enum) (Variables|/Game/_Assets/Blueprints/Characters/Cube.Cube_C|GetPathingStyle _ascube) "NewEnumerator2")
            (Utilities|Array|Reverse (Variables|/Game/_Assets/Blueprints/Characters/Cube.Cube_C|GetPatrolPath _ascube))
            (Class|BTFunctionLibrary|SetBlackboardValueasObject (Variables|Default|GetKey) (Utilities|Array|Get(acopy) (Variables|/Game/_Assets/Blueprints/Characters/Cube.Cube_C|GetPatrolPath _ascube) _output_get) :!label _label)
            (elif (Utilities|Enum|Equal(Enum) (Variables|/Game/_Assets/Blueprints/Characters/Cube.Cube_C|GetPathingStyle _ascube) "NewEnumerator1")
              (Transformation|SetActorLocation _ascube (Transformation|GetActorLocation (Utilities|Array|Get(acopy) (Variables|/Game/_Assets/Blueprints/Characters/Cube.Cube_C|GetPatrolPath _ascube) _output_get)) false false)
              (goto _label)
              (elif (Utilities|Enum|Equal(Enum) (Variables|/Game/_Assets/Blueprints/Characters/Cube.Cube_C|GetPathingStyle _ascube) "NewEnumerator0")
                (goto _label)
                (else
                  (Variables|/Game/_Assets/Blueprints/Characters/Cube.Cube_C|SetState _ascube "NewEnumerator3"))))))))))