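; Behavior tree task that makes an AI-controlled Cube pawn tackle by dashing toward a blackboard target actor.
; On execute it casts the owner to get the pawn and sets its state, failing if either cast fails.
; Tick faces the target and starts the dash, then stops it and succeeds after roughly a fifth of a second.
; Aborting stops the dash and resets the timer.
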(event EventReceiveAbort
  (params (OwnerActor :type Actor%20Object%20Reference))
  (Default|StopDash (Variables|Default|GetAIPawn))
  (Variables|Default|SetTickCount 0.0)
  (Class|BTTaskBlueprintBase|FinishAbort))

(event EventReceiveExecute
  (params (OwnerActor :type Actor%20Object%20Reference))
  (bind _asaicontroller (Utilities|Casting|CastToAIController OwnerActor)
    (:then
      (bind _ascube (Utilities|Casting|CastToCube (Pawn|GetControlledPawn _asaicontroller))
        (:then
          (bind _output_get (Variables|Default|SetAIPawn _ascube))
          (Variables|/Game/_Assets/Blueprints/Characters/Cube.Cube_C|SetState _output_get "NewEnumerator1"))
        (:CastFailed
          (Development|PrintString "bad pawn")
          (AI|BehaviorTree|FinishExecute false :!label _label))))
    (:CastFailed
      (Development|PrintString "bad parent")
      (goto _label))))

(event EventTick
  (params (OwnerActor :type Actor%20Object%20Reference) (DeltaSeconds :type Float%20%28single-precision%29))
  (bind _aipawn (Variables|Default|GetAIPawn))
  (bind _key (Variables|Default|GetKey))
  (bind _returnvalue (AI|BehaviorTree|GetBlackboardValueasActor _key))
  (bind _returnvalue_2 (Transformation|GetActorLocation _aipawn))
  (bind _returnvalue_3 (Transformation|GetActorLocation _returnvalue))
  (bind _returnvalue_4 (Math|Rotator|FindLookatRotation _returnvalue_2 _returnvalue_3))
  (if (== (Variables|Default|GetTickCount) 0.0)
    (Transformation|SetActorRotation _aipawn _returnvalue_4)
    (Default|StartDash (Variables|Default|GetAIPawn) _returnvalue_4)
    (Variables|Default|SetTickCount (+ DeltaSeconds (Variables|Default|GetTickCount)))
    (elif (> (Variables|Default|GetTickCount) 0.2)
      (Default|StopDash (Variables|Default|GetAIPawn))
      (Variables|Default|SetTickCount 0.0)
      (AI|BehaviorTree|FinishExecute true)
      (else
        (Variables|Default|SetTickCount (+ DeltaSeconds (Variables|Default|GetTickCount)))))))