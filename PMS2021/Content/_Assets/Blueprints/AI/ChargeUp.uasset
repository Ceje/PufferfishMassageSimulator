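; Behavior Tree task that plays a timed charge-up on the AI-controlled Cube pawn by spinning its cube component.
; On execute it caches the pawn and sets its state, failing if the controller or pawn cast fails.
; Tick accumulates time to drive yaw through ChangeColor, which only rotates despite its name, then succeeds after about two seconds.
; Abort resets the rotation and timer.
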(event EventReceiveExecute
  (params (OwnerActor :type Actor%20Object%20Reference))
  (bind _asaicontroller (Utilities|Casting|CastToAIController OwnerActor)
    (:then
      (bind _ascube (Utilities|Casting|CastToCube (Pawn|GetControlledPawn _asaicontroller))
        (:then
          (bind _output_get (Variables|Default|SetActor _ascube))
          (Variables|/Game/_Assets/Blueprints/Characters/Cube.Cube_C|SetState _output_get "NewEnumerator0"))
        (:CastFailed
          (Development|PrintString "bad pawn")
          (AI|BehaviorTree|FinishExecute false :!label _label))))
    (:CastFailed
      (Development|PrintString "bad parent")
      (goto _label))))

(event EventTick
  (params (OwnerActor :type Actor%20Object%20Reference) (DeltaSeconds :type Float%20%28single-precision%29))
  (bind _output_get (Variables|Default|SetDuration (+ DeltaSeconds (Variables|Default|GetDuration))))
  (if (> _output_get 2.0)
    (Variables|Default|SetDuration 0.0)
    (AI|BehaviorTree|FinishExecute true)
    (else
      (CallFunction|ChangeColor _output_get))))

(event EventReceiveAbort
  (params (OwnerActor :type Actor%20Object%20Reference))
  (CallFunction|ChangeColor 0.0)
  (Variables|Default|SetDuration 0.0)
  (Class|BTTaskBlueprintBase|FinishAbort))

(fn ChangeColor
  (params (Time :type Float%20%28single-precision%29))
  (Transformation|SetRelativeRotation (Variables|/Game/_Assets/Blueprints/Characters/Cube.Cube_C|GetCube (Variables|Default|GetActor)) (Math|Rotator|MakeRotator 0.0 0.0 (* 360 Time)) false false))