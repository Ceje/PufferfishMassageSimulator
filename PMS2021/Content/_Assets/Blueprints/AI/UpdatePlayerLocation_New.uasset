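; Behavior tree service that, on activation, writes a sidestep location relative to the player into a blackboard vector key, despite its name suggesting the player's location.
; It finds the look-at rotation from the controlled pawn to player 0, adds 90 degrees of yaw, and offsets the pawn's location a short fixed distance along that direction.
; The point is computed once per activation, with no periodic update.
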(event EventReceiveActivationAI
  (params (OwnerController :type AI%20Controller%20Object%20Reference) (ControlledPawn :type Pawn%20Object%20Reference))
  (bind _returnvalue (Transformation|GetActorLocation ControlledPawn))
  (bind _returnvalue_2 (Game|Player|GetPlayerPawn 0))
  (bind _returnvalue_3 (Transformation|GetActorLocation _returnvalue_2))
  (bind _returnvalue_4 (Math|Rotator|FindLookatRotation _returnvalue _returnvalue_3))
  (bind (_roll _pitch _yaw) (Math|Rotator|BreakRotator _returnvalue_4))
  (AI|BehaviorTree|SetBlackboardValueasVector (Variables|Default|Getkey) (+ _returnvalue (* (Math|Vector|GetForwardVector (Math|Rotator|MakeRotator _roll _pitch (+ _yaw 9e+01))) 1e+02))))