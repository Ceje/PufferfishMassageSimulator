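; Level streamer actor that requests loading and unloading of a chosen level as the player pawn enters and leaves its overlap area.
; It caches the PMSGameState at BeginPlay and delegates stream and unstream requests to it.
; The spawn transform comes from an optional SpawnReference actor, falling back to its own transform.
; When SelfPreserving is set, it also requests the level at BeginPlay, though overlap exit still unloads it.
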(event Custom|LoadLevel
  (bind _spawnreference (Variables|Default|GetSpawnReference))
  (Default|StreamLevelRequest (Variables|Default|GetGameStateRef) (Variables|Default|GetLevelToStream) (select (Utilities|IsValid _spawnreference) (Transformation|GetActorTransform _spawnreference) (Transformation|GetActorTransform))))

(event Collision|EventActorBeginOverlap
  (params (OtherActor :type Actor%20Object%20Reference))
  (if (== OtherActor (Game|Player|GetPlayerPawn 0))
    (CallFunction|LoadLevel)))

(event Collision|EventActorEndOverlap
  (params (OtherActor :type Actor%20Object%20Reference))
  (if (== OtherActor (Game|Player|GetPlayerPawn 0))
    (Default|UnstreamLevelRequest (Variables|Default|GetGameStateRef) (Variables|Default|GetLevelToStream))))

(event EventBeginPlay
  (bind _aspmsgame_state (Utilities|Casting|CastToPMSGameState (Game|GetGameState))
    (:then
      (Variables|Default|SetGameStateRef _aspmsgame_state)
      (if (Variables|Default|GetSelfPreserving)
        (CallFunction|LoadLevel)))
    (:CastFailed
      (Development|PrintString "Level Streamer Faild to Retrieve Game State"))))

(fn ConstructionScript)